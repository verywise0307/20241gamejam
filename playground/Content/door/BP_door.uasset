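; BP_door is a level-exit door that opens and becomes usable once the level's BP_mob reports its Over flag.
; Tick looks up the BP_mob actor every frame and, while Over is set, snaps the door to a fixed open rotation.
; A FirstPersonCharacter overlapping the door checks the same flag and, if set, loads the level named by the Mapname variable.
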(event EventBeginPlay)

(event Collision|EventActorBeginOverlap
  (params (OtherActor :type Actor%20Object%20Reference))
  (Utilities|Casting|CastToFirstPersonCharacter OtherActor)
  (if (Variables|/Game/mob/BP_mob.BP_mob_C|Getover (stale EventTick _returnvalue))
    (Game|OpenLevel(byName) (Utilities|String|StringToName (Variables|Default|Getmapname)))))

(event EventTick
  (params (DeltaSeconds :type Float%20%28single-precision%29))
  (bind _returnvalue (Actor|GetActorOfClass "/Game/mob/BP_mob.BP_mob_C"))
  (if (Variables|/Game/mob/BP_mob.BP_mob_C|Getover _returnvalue)
    (Transformation|SetActorRotation "0,-70.000000, 0")))

(fn ConstructionScript)