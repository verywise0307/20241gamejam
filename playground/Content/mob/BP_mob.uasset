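; Red-light/green-light style mob that cycles between safe and watching phases through the shared GI game instance's IsIdle flag.
; The safe phase shows a white light and bubble effect for a random delay.
; Watching begins with a two-second grace delay, then turns the light red, faces and approaches the player unless Stop is set, and flags GameOver if the player moves.
; Alerting also sets GI.Die and decrements NodeChance.
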(event Custom|red%20light
  (Rendering|Components|Light|SetLightColor (Variables|Default|GetPointLight) "(R=1.000000,G=0.019486,B=0.000000,A=1.000000)" true)
  (bind _asfirst_person_character (Utilities|Casting|CastToFirstPersonCharacter (Game|GetPlayerCharacter 0)))
  (if (>= (Math|Vector|VectorLength (Transformation|GetVelocity _asfirst_person_character)) 2e+01)
    (Variables|/Game/GI.GI_C|Setgame%20over (stale EventBeginPlay _asgi) true)))

(event Custom|white%20light
  (Rendering|Components|Light|SetLightColor (Variables|Default|GetPointLight) "(R=1.000000,G=1.000000,B=1.000000,A=1.000000)" true))

(event Custom|idle
  (Utilities|FlowControl|Delay (Math|Conversions|ToFloat(Integer) (Math|Random|RandomIntegerinRange 7 12)))
  (bind _asgi (Utilities|Casting|CastToGI (Game|GetGameInstance)))
  (Variables|/Game/GI.GI_C|SetIsIdle (stale EventBeginPlay _asgi) false)
  (if (== (Variables|/Game/GI.GI_C|Getnum_X _asgi) 2)
    (Variables|/Game/GI.GI_C|Setnum_X _asgi 0)))

(event Custom|not%20idle
  (if (Variables|Default|Getnot)
    (Utilities|FlowControl|Sequence
      (:then_0
        (Variables|Default|Setnot false)
        (bind _output_get (Variables|Default|Settime (Math|Random|RandomIntegerinRange 5 10)))
        (Utilities|FlowControl|Delay (Math|Conversions|ToFloat(Integer) _output_get))
        (Variables|/Game/GI.GI_C|SetIsIdle (stale EventBeginPlay _asgi) true)
        (Variables|Default|Setalert false)
        (CallFunction|Idle)
        (Variables|Default|Setnot true))
      (:then_1
        (Rendering|SetVisibility (Variables|Default|Getbubblebubble) true false)
        (Utilities|FlowControl|Delay (Math|Conversions|ToFloat(Integer) (* (/ (Variables|Default|Gettime) 6) 2)))
        (Development|PrintString "작아져라")
        (Effects|Components|ParticleSystem|SetFloatParameter (Variables|Default|Getbubblebubble) "SpawnRate" 2e+01)
        (Utilities|FlowControl|Delay (Math|Conversions|ToFloat(Integer) (* (/ (Variables|Default|Gettime) 6) 2)))
        (Development|PrintString "작아져라!!!!!")
        (Effects|Components|ParticleSystem|SetFloatParameter (Variables|Default|Getbubblebubble) "Spawn Rate" 1e+01)
        (Utilities|FlowControl|Delay (Math|Conversions|ToFloat(Integer) (* (/ (Variables|Default|Gettime) 6) 2)))
        (Effects|Components|ParticleSystem|SetFloatParameter (Variables|Default|Getbubblebubble) "Spawn Rate" 3e+01)
        (Rendering|SetVisibility (Variables|Default|Getbubblebubble) false false)))))

(event EventBeginPlay
  (bind _asgi (Utilities|Casting|CastToGI (Game|GetGameInstance))))

(event Collision|EventActorBeginOverlap
  (params (OtherActor :type Actor%20Object%20Reference)))

(event EventTick
  (params (DeltaSeconds :type Float%20%28single-precision%29))
  (Utilities|FlowControl|Sequence
    (:then_0
      (if (Variables|/Game/GI.GI_C|GetIsIdle (stale EventBeginPlay _asgi))
        (if (Variables|Default|Getalert)
          (CallFunction|RedLight)
          (bind _output_get (Variables|Default|Setrotation (Math|Rotator|MakeRotator 0.0 0.0 (.Yaw (Math|Rotator|BreakRotator (Math|Rotator|FindLookatRotation (Transformation|GetActorLocation) (Transformation|GetActorLocation (Game|GetPlayerCharacter 0))))))))
          (Transformation|SetActorRotation _output_get)
          (bind _returnvalue (Actor|GetActorOfClass "/Game/FirstPersonBP/Blueprints/FirstPersonCharacter.FirstPersonCharacter_C"))
          (if (not (Variables|/Game/FirstPersonBP/Blueprints/FirstPersonCharacter.FirstPersonCharacter_C|Getstop _returnvalue))
            (Transformation|AddActorWorldOffset (* (Transformation|GetActorForwardVector) (* (Variables|Default|Getspeed) (Utilities|Time|GetWorldDeltaSeconds)))))
          (else
            (Utilities|FlowControl|Delay 2.0)
            (Variables|Default|Setalert true)
            (Variables|/Game/GI.GI_C|Setdie (stale EventBeginPlay _asgi) true)
            (Variables|/Game/GI.GI_C|Setnode_chance (stale EventBeginPlay _asgi) (- (Variables|/Game/GI.GI_C|Getnode_chance (stale EventBeginPlay _asgi)) 1))))
        (else
          (Variables|/Game/GI.GI_C|Setdie (stale EventBeginPlay _asgi) false)
          ;[1 1 1] 고개 숙이고 있을 때
          (CallFunction|WhiteLight)
          (CallFunction|NotIdle))))))

(fn ConstructionScript)